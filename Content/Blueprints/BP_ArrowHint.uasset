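; BP_ArrowHint is an arrow that lights up as a hint for the player, meant especially for early and tutorial levels.
; OnCollision, triggered when the arrow is scanned, sets both mesh material slots to MI_GlowyWhite if AllowOnDetected passes its check.
; For stuck players, BeginPlay can also call OnCollision after DelayBeforeShowingHint when AllowsHint passes, so that timed reveal still depends on AllowOnDetected.
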(event `self.ReceiveBeginPlay`
  ; In case we wanna show it when the player is stuck, add a timer for it to show it after X seconds
  (`parent.ReceiveBeginPlay`)
  (`self.AllowsHint`
    (:`then`
      (`KismetSystemLibrary.Delay` (`self.DelayBeforeShowingHint`))
      (`self.onCollision` null))
    (:`else`)))

(event `/Game/Blueprints/Intefaces/BPI_ChangeSphereCollor.onCollision`
  (params (`Scanner Point` :type "/Game/Blueprints/BP_ScannerPoint Object Reference") (`Spawn Point` :type "Vector Structure"))
  (bind _mesh (`self.Mesh`))
  ; When scanned, show the arrow to help the plaer (specially for incital lvls and tutorialization)
  (`self.AllowOnDetected`
    (:`then`
      (`PrimitiveComponent.SetMaterial` _mesh 0 "/Game/Materials/MI_GlowyWhite.MI_GlowyWhite")
      (`PrimitiveComponent.SetMaterial` _mesh 1 "/Game/Materials/MI_GlowyWhite.MI_GlowyWhite"))
    (:`else`)))

(fn `UserConstructionScript`
  (`parent.UserConstructionScript`))