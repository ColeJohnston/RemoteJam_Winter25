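; BP_LoseZones is a hazard actor that makes the player lose on contact with its mesh.
; Its mesh hit event checks for player character 0, then adds a W_LoseScreen widget, switches input to UI only and shows the cursor.
; Its scanner collision event only calls the parent implementation, commented as showing the scan dots in red.
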(event `/Game/Blueprints/Intefaces/BPI_ChangeSphereCollor.onCollision`
  (params (`Scanner Point` :type "/Game/Blueprints/BP_ScannerPoint Object Reference") (`Spawn Point` :type "Vector Structure"))
  ; Show the dots in red when scanned
  (`parent.onCollision` `Scanner Point` `Spawn Point`))

(event `self.Mesh.OnComponentHit`
  (params (HitComponent :type "PrimitiveComponent Object Reference") (OtherActor :type "Actor Object Reference") (OtherComp :type "PrimitiveComponent Object Reference") (NormalImpulse :type "Vector Structure") (Hit :type "HitResult Structure (by ref)"))
  ; When hit the mesh, show lose square, try again
  (if (== OtherActor (`GameplayStatics.GetPlayerCharacter` 0))
    (bind _returnvalue (`|CreateWidget` "/Game/UI/W_LoseScreen.W_LoseScreen_C"))
    (`UserWidget.AddToViewport` _returnvalue 0)
    (`WidgetBlueprintLibrary.SetInputMode_UIOnlyEx` (`GameplayStatics.GetPlayerController` 0) null "DoNotLock" true)
    (set `PlayerController.bShowMouseCursor` true (`GameplayStatics.GetPlayerController` 0))))

(fn `UserConstructionScript`
  (`parent.UserConstructionScript`))