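; BP_NextLevelSquare is an end-of-level trigger that shows the next-level screen when the player reaches it.
; On BeginPlay it pre-creates a W_NextLevelScreen widget and passes it the LevelNumber.
; When the player character overlaps its Box, it removes all widgets, waits one tick, adds that screen to the viewport and sets LevelBeat to true.
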(event `self.ReceiveBeginPlay`
  (bind _returnvalue (`|CreateWidget` "/Game/UI/W_NextLevelScreen.W_NextLevelScreen_C" (`GameplayStatics.GetPlayerController` 0)))
  (bind _output_get (set `self.NextLevelScreen` _returnvalue))
  (set `/Game/UI/W_NextLevelScreen.LevelNumber` (`self.LevelNumber`) _output_get))

(event `self.Box.OnComponentBeginOverlap`
  (params (OverlappedComponent :type "PrimitiveComponent Object Reference") (OtherActor :type "Actor Object Reference") (OtherComp :type "PrimitiveComponent Object Reference") (OtherBodyIndex :type Integer) (bFromSweep :type Boolean) (SweepResult :type "HitResult Structure (by ref)"))
  (if (== OtherActor (`GameplayStatics.GetPlayerCharacter` 0))
    (`WidgetLayoutLibrary.RemoveAllWidgets`)
    (`KismetSystemLibrary.DelayUntilNextTick`)
    (`UserWidget.AddToViewport` (`self.NextLevelScreen`) 0)
    (set `self.LevelBeat?` true)))

(fn `UserConstructionScript`)