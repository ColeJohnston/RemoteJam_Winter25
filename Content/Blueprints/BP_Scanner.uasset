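; BP_Scanner runs a timed screen scan that marks surfaces in the level with dots at line trace hit locations.
; ScanScreen starts the widget animation, scaled to the scan time, and Tick advances the scan row by row, disabling player input until it finishes.
; Each row sweeps an arrow component across a yaw and pitch grid, tracing on Visibility.
; Hits go to a BP_ScannerPoint instancer spawned on BeginPlay, so levels need none placed.
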(event `self.ReceiveTick`
  (params (DeltaSeconds :type "Float (single-precision)"))
  ;[0.15 0.15 0.15 0.5 34] Keep track of time scanning
  (set `self.Delta Seconds` DeltaSeconds)
  (if (`self.Scanning`)
    (bind _output_get (set `self.ElapsedTime` (+ (`self.ElapsedTime`) (`self.Delta Seconds`))))
    (bind _returnvalue (`KismetMathLibrary.FClamp` (/ _output_get (`self.ScanTime`))))
    ;[0.15 0.15 0.15 0.5 34] After enough time, scan another row on Y axis
    (set `self.ScanAlpha` _returnvalue)
    (`/Game/UI/W_Scanner.SetPositionOfScan` (`self.Scanner Widget`))
    (if (> (`KismetMathLibrary.FFloor` (* _returnvalue (`self.YNumberOfDots`))) (`self.YScanCounter`))
      (`self.ScanY`)
      ;[0.15 0.15 0.15 0.5 34] If scanned enough, reset everything back to initial values
      (bind _result (`/Engine/EditorBlueprintResources/StandardMacros.IncrementInt` (`self.YScanCounter`))
        (:`  `
          (if (== _result (`self.YNumberOfDots`))
            (set `self.YScanCounter` 0)
            (set `self.ElapsedTime` 0.0)
            (set `self.Scanning` false)
            (`Actor.EnableInput` (`GameplayStatics.GetPlayerCharacter` 0) (`GameplayStatics.GetPlayerController` 0))))))))

(event `self.ReceiveBeginPlay`
  ;[0.15 0.15 0.15 0.5 34] This is what spawns the dot spawner. No need to put one in every level
  (bind _returnvalue (`|SpawnActorFromClass` "/Game/Blueprints/BP_ScannerPoint.BP_ScannerPoint_C" (`KismetMathLibrary.MakeTransform` (0.0 0.0 -100000000.0)) "Undefined" "MultiplyWithRoot" null null))
  (set `self.ScanerPointInstancer` _returnvalue))

(event `ScanY`
  (bind _arrow (`self.Arrow`))
  (bind _returnvalue (`SceneComponent.K2_GetComponentLocation` _arrow))
  (`Actor.DisableInput` (`GameplayStatics.GetPlayerCharacter` 0) (`GameplayStatics.GetPlayerController` 0))
  (for _index (range (`self.XNumberOfDots`))
    (`SceneComponent.K2_SetRelativeRotation` (`self.Arrow`) (`KismetMathLibrary.MakeRotator` 0.0 (- (`self.YDegrees`) (* (`self.YScanCounter`) (/ (* (`self.YDegrees`) 2) (- (`self.YNumberOfDots`) 1)))) (- (`self.XDegrees`) (* _index (/ (* (`self.XDegrees`) 2) (- (`self.XNumberOfDots`) 1))))) false false)
    ;[0.15 0.15 0.15 0.5 34] Line trace area and spawn a dot where line trace hits
    (bind _outhit (`KismetSystemLibrary.LineTraceSingle` :`Start` _returnvalue :`End` (+ _returnvalue (* (`SceneComponent.GetForwardVector` _arrow) 100000000.0)) :`TraceChannel` "TraceTypeQuery1" :`TraceColor` (struct :`R` 1.0)))
    (`/Game/Blueprints/BP_ScannerPoint.SpawnScannerPoint` (`self.ScanerPointInstancer`) (`.Location` (`GameplayStatics.BreakHitResult` _outhit)))))

(event `ScanScreen`
  (params (Arrow :type "SceneComponent Object Reference") (ScannerWidget :type "/Game/UI/W_Scanner Object Reference"))
  ;[0.15 0.15 0.15 0.5 34] Initialize screen scanning
  (set `self.Arrow` Arrow)
  (bind _output_get (set `self.Scanner Widget` ScannerWidget))
  (`UserWidget.PlayAnimation` _output_get (`/Game/UI/W_Scanner.ScanScreen` _output_get) 0.0 1 "Forward" (/ 1.0 (`self.ScanTime`)) false)
  (set `self.Scanning` true))