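; BP_ScannerPoint is an actor that renders the dots left by the player's scanner as instances on a single instanced mesh component.
; SpawnScannerPoint adds a world-space instance at the given location, scaled uniformly by DotSize.
; The dot cap comes from the first-person character's BPScanner, multiplying allowed scans by dots per scan.
; When a new instance's index reaches that cap, instance zero is removed, intended to clear dots oldest first.
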(event `self.ReceiveBeginPlay`
  ; Spawn scanner point and if there is more than 3 scans worth of dots on screen, remove dots in order of spawn.
  (bind _returnvalue (`GameplayStatics.GetActorOfClass` "/Game/FirstPerson/Blueprints/BP_FirstPersonCharacter.BP_FirstPersonCharacter_C")))

(event `SpawnScannerPoint`
  (params (SpawnPoint :type "Vector Structure"))
  (bind _dotsize (`self.DotSize`))
  ; Spawn scanner point and if there is more than 3 scans worth of dots on screen, remove dots in order of spawn.
  (bind _returnvalue (`InstancedStaticMeshComponent.AddInstance` (`self.ScannerPoint`) (`KismetMathLibrary.MakeTransform` SpawnPoint (struct) (`KismetMathLibrary.MakeVector` _dotsize _dotsize _dotsize)) true))
  (bind _bp_scanner (`/Game/FirstPerson/Blueprints/BP_FirstPersonCharacter.BP_Scanner` (stale `self.ReceiveBeginPlay` _returnvalue)))
  (if (>= _returnvalue (* (`/Game/Blueprints/BP_Scanner.MaxScansAllowed` _bp_scanner) (`/Game/Blueprints/BP_Scanner.XNumberOfDots` _bp_scanner) (`/Game/Blueprints/BP_Scanner.YNumberOfDots` _bp_scanner)))
    (`InstancedStaticMeshComponent.RemoveInstance` (`self.ScannerPoint`) 0)))

(fn `UserConstructionScript`)