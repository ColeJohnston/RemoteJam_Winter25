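; BP_WinSquare is a trigger box that ends the run with a win screen when the player walks into it.
; It creates the W_WinScreen widget on BeginPlay and adds it to the viewport when the player character overlaps the Box.
; The overlap also switches input to UI only, shows the mouse cursor and stops the BP_FirstPersonCharacter countdown by clearing its ReduceTime timer.
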(event `self.ReceiveBeginPlay`
  ; Initialize win screen and save as variable
  (bind _returnvalue (`|CreateWidget` "/Game/UI/W_WinScreen.W_WinScreen_C"))
  (set `self.WinScreen` _returnvalue))

(event `self.Box.OnComponentBeginOverlap`
  (params (OverlappedComponent :type "PrimitiveComponent Object Reference") (OtherActor :type "Actor Object Reference") (OtherComp :type "PrimitiveComponent Object Reference") (OtherBodyIndex :type Integer) (bFromSweep :type Boolean) (SweepResult :type "HitResult Structure (by ref)"))
  ; When player overlaps with the box, set input to ui only and add win screen
  (if (== OtherActor (`GameplayStatics.GetPlayerCharacter` 0))
    (`UserWidget.AddToViewport` (`self.WinScreen`) 0)
    (`WidgetBlueprintLibrary.SetInputMode_UIOnlyEx` (`GameplayStatics.GetPlayerController` 0) (`self.WinScreen`) "DoNotLock" true)
    (set `PlayerController.bShowMouseCursor` true (`GameplayStatics.GetPlayerController` 0))
    (bind _asbp_first_person_character (cast `/Game/FirstPerson/Blueprints/BP_FirstPersonCharacter` (`GameplayStatics.GetPlayerCharacter` 0)))
    (`KismetSystemLibrary.K2_ClearTimer` _asbp_first_person_character "ReduceTime")))

(fn `UserConstructionScript`)